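; HUD Blueprint that draws a lock-on marker over the player's current target.
; BeginPlay caches the player character, and Tick sets the marker size from its lock state, dropping it to zero when not locked.
; DrawHUD projects the locked actor's world location to screen space and draws a white target texture there with a small fixed pixel offset.
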(event EventBeginPlay
  (bind _asplayer_character_1 (Utilities|Casting|CastToPlayerCharacter1 (Game|GetPlayerCharacter 0)))
  (Variables|Default|SetCharacterRef _asplayer_character_1))

(event EventTick
  (params (DeltaSeconds :type Float%20%28single-precision%29))
  (bind _characterref (Variables|Default|GetCharacterRef))
  (if (and (Variables|/Game/Blueprints/Character/PlayerCharacter1.PlayerCharacter1_C|GetTargetLocked _characterref) (Utilities|IsValid (Variables|/Game/Blueprints/Character/PlayerCharacter1.PlayerCharacter1_C|GetTargetLockActor _characterref)))
    (Variables|Default|SetTargetScale 12.0)
    (else
      (Variables|Default|SetTargetScale 0.0))))

(event EventDrawHUD
  (params (SizeX :type Integer) (SizeY :type Integer))
  (bind _returnvalue (Game|GetPlayerController 0))
  (bind _characterref (Variables|Default|GetCharacterRef))
  (bind _targetscale (Variables|Default|GetTargetScale))
  (bind _targetlockactor (Variables|/Game/Blueprints/Character/PlayerCharacter1.PlayerCharacter1_C|GetTargetLockActor _characterref))
  (bind _returnvalue_2 (Transformation|GetActorLocation _targetlockactor))
  (bind _screenlocation (Class|PlayerController|ProjectWorldLocationtoScreen _returnvalue _returnvalue_2 false))
  (Utilities|IsValid _targetlockactor
    (:Is%20Valid
      (Canvas|DrawTexture "/Game/Assets/Images/TargetWhite.TargetWhite" (- (.x _screenlocation) 6.0) (- (.y _screenlocation) 2e+01) _targetscale _targetscale 0.0 0.0 1.0 1.0 "(R=1.000000,G=1.000000,B=1.000000,A=1.000000)"))))

(fn ConstructionScript)