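; A sword lying on the ground that the player picks up through a scripted animation.
; Overlapping its sphere shows a prompt widget and enables the interact input, which works only if the player has no sword.
; Interacting locks player input, toggles the camera, snaps the character beside the sword and plays the pickup animation.
; Timed delays swap in a temporary socket-attached sword, call PickupSword, restore control and destroy the actor.
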(event OnComponentEndOverlap(Sphere)
  (params (OverlappedComponent :type Primitive%20Component%20Object%20Reference) (OtherActor :type Actor%20Object%20Reference) (OtherComp :type Primitive%20Component%20Object%20Reference) (OtherBodyIndex :type Integer))
  (Utilities|Casting|CastToPlayerCharacter OtherActor)
  (Input|DisableInput (Game|GetPlayerController 0))
  (Rendering|SetVisibility (Variables|Default|GetWidget) false false))

(event OnComponentBeginOverlap(Sphere)
  (params (OverlappedComponent :type Primitive%20Component%20Object%20Reference) (OtherActor :type Actor%20Object%20Reference) (OtherComp :type Primitive%20Component%20Object%20Reference) (OtherBodyIndex :type Integer) (bFromSweep :type Boolean) (SweepResult :type Hit%20Result%20Structure%20%28by%20ref%29))
  (Utilities|Casting|CastToPlayerCharacter OtherActor)
  (Input|EnableInput (Game|GetPlayerController 0))
  (Rendering|SetVisibility (Variables|Default|GetWidget) true false))

(event Input|ActionEvents|InputActionInterect
  (params (Key :type Key%20Structure :default "None"))
  (bind _returnvalue (Game|GetPlayerController 0))
  (bind _returnvalue_2 (Game|GetPlayerCharacter 0))
  (bind _returnvalue_3 (Transformation|GetActorLocation))
  (bind _returnvalue_4 (Game|GetPlayerCharacter 0))
  (bind _returnvalue_5 (Game|GetPlayerCharacter 0))
  (bind _asplayer_character (Utilities|Casting|CastToPlayerCharacter _returnvalue_2))
  (bind _asplayer_character_2 (Utilities|Casting|CastToPlayerCharacter _returnvalue_5))
  (bind _asplayer_character_3 (Utilities|Casting|CastToPlayerCharacter _returnvalue_4))
  (bind _mesh (Variables|/Script/Engine.Character|GetMesh _asplayer_character_3))
  (:Pressed
    (if (not (Utilities|IsValid (Variables|/Game/Blueprints/Character/PlayerCharacter.PlayerCharacter_C|GetSwordRef _asplayer_character)))
      (Input|DisableInput (Game|GetPlayerController 0))
      (Rendering|SetVisibility (Variables|Default|GetWidget) false false)
      (Default|SetCamera _asplayer_character)
      (Input|DisableInput _returnvalue_4 _returnvalue)
      (Transformation|SetActorLocation _asplayer_character_3 (Math|Vector|MakeVector (- (.x _returnvalue_3) 5e+01) (- (.y _returnvalue_3) 15.0) (+ (.z _returnvalue_3) 1e+02)) false false)
      (Transformation|SetActorRotation _asplayer_character_3 (Transformation|GetActorRotation))
      (Components|Animation|PlayAnimation _mesh "/Game/Assets/Mannequin/Animations/Sword_Animations/Interect/PickupSwordFromGround.PickupSwordFromGround" false)
      (Utilities|FlowControl|Delay 1.5)
      (Rendering|SetVisibility (Variables|Default|GetMesh) false false)
      (bind _returnvalue_6 (Game|SpawnActorfromClass "/Game/Blueprints/Weapons/ShortSword_BP.ShortSword_BP_C" (Math|Transform|MakeTransform "0, 0, 0") "Undefined" 0 0))
      (bind _output_get (Variables|Default|SetRef _returnvalue_6))
      (Collision|SetCollisionEnabled (Variables|/Game/Blueprints/Weapons/SwordParent_BP.SwordParent_BP_C|GetSphere _returnvalue_6) "NoCollision")
      (Transformation|AttachComponentToComponent _output_get _mesh "PickUpAnimSocket" "SnapToTarget" "SnapToTarget" "KeepRelative" true)
      (Utilities|FlowControl|Delay 4.0)
      (Actor|DestroyActor (Variables|Default|GetRef))
      (Default|PickupSword (.AsPlayer%20Character (Utilities|Casting|CastToPlayerCharacter _returnvalue_5)))
      (Utilities|FlowControl|Delay 1.5)
      (Input|EnableInput _returnvalue_5 _returnvalue)
      (Components|Animation|SetAnimationMode (Variables|/Script/Engine.Character|GetMesh _asplayer_character_2) "AnimationBlueprint")
      (Default|SetCamera _asplayer_character_2)
      (Actor|DestroyActor))))

(fn ConstructionScript)