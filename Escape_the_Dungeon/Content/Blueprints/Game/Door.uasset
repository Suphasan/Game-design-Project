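; Door actor that slides open vertically when PlayerCharacter1 enters its Box trigger and reverses when the player leaves.
; A timeline plays or reverses on overlap events, driving the StaticMesh's relative Z location.
; When NeedSwordToOpen is set, both opening and closing require the player to have a valid SwordRef.
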(event OnComponentBeginOverlap(Box)
  (params (OverlappedComponent :type Primitive%20Component%20Object%20Reference) (OtherActor :type Actor%20Object%20Reference) (OtherComp :type Primitive%20Component%20Object%20Reference) (OtherBodyIndex :type Integer) (bFromSweep :type Boolean) (SweepResult :type Hit%20Result%20Structure%20%28by%20ref%29))
  (bind _asplayer_character_1 (Utilities|Casting|CastToPlayerCharacter1 OtherActor))
  (if (Variables|Default|GetNeedSwordToOpen?)
    (if (Utilities|IsValid (Variables|/Game/Blueprints/Character/PlayerCharacter1.PlayerCharacter1_C|GetSwordRef _asplayer_character_1))
      (bind _newtrack_0 (Timeline|Timeline_0 Play)
        (:Update
          (Transformation|SetRelativeLocation (Variables|Default|GetStaticMesh) (Math|Vector|MakeVector 0.0 0.0 _newtrack_0) false false))))
    (else
      (Timeline|Timeline_0 Play))))

(event OnComponentEndOverlap(Box)
  (params (OverlappedComponent :type Primitive%20Component%20Object%20Reference) (OtherActor :type Actor%20Object%20Reference) (OtherComp :type Primitive%20Component%20Object%20Reference) (OtherBodyIndex :type Integer))
  (bind _asplayer_character_1 (Utilities|Casting|CastToPlayerCharacter1 OtherActor))
  (if (Variables|Default|GetNeedSwordToOpen?)
    (if (Utilities|IsValid (Variables|/Game/Blueprints/Character/PlayerCharacter1.PlayerCharacter1_C|GetSwordRef _asplayer_character_1))
      (bind _newtrack_0 (Timeline|Timeline_0 Reverse)
        (:Update
          (Transformation|SetRelativeLocation (Variables|Default|GetStaticMesh) (Math|Vector|MakeVector 0.0 0.0 _newtrack_0) false false))))
    (else
      (Timeline|Timeline_0 Reverse))))

(fn ConstructionScript)