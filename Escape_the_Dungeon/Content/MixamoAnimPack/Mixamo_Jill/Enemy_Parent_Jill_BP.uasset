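; Parent Blueprint for a melee enemy that chases the player and attacks with a sword spawned onto its Equip socket.
; Pawn sensing latches chasing through AIMoveTo, while a short forward trace each Tick triggers attack montages, gated by CanAttack.
; DealingDamage updates the health bar widget, plays a sound and briefly blocks new move orders.
; At zero health, it ragdolls, hides the bar, disables capsule collision and pauses the sword's AttackTrace timer.
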(event OnSeePawn(PawnSensing)
  (params (Pawn :type Pawn%20Object%20Reference))
  ;[1 1 1] Event See
  (Variables|Default|SetEnemySeePlayer true))

(event Custom|Attack
  ;[1 1 1] Event Attack
  (if (and (not (Variables|Default|GetEnemyDeath)) (Variables|Default|GetCanAttack?))
    (Variables|Default|SetCanAttack? false)
    (bind _returnvalue (Animation|PlayAnimMontage (Utilities|Array|Get(acopy) (Variables|Default|GetAttacks) (Math|Random|RandomInteger 1)) 1.0 "None"))
    (Utilities|FlowControl|Delay _returnvalue)
    (Variables|Default|SetCanAttack? true)))

(event Custom|AddWeapon
  ;[1 1 1] Add Enemy Weapon
  (bind _returnvalue (Game|SpawnActorfromClass "/Game/Blueprints/Enemys/EnemySword_BP.EnemySword_BP_C" (Math|Transform|MakeTransform "0, 0, 0") "Undefined" 0 0))
  (bind _output_get (Variables|Default|SetEnemySwordRef _returnvalue))
  (Transformation|AttachComponentToComponent _output_get (Variables|Character|GetMesh) "Equip" "SnapToTarget" "SnapToTarget" "KeepRelative" true))

(event Custom|MoveToPlayer
  ;[1 1 1] MoveToPlayer
  (if (Variables|Default|GetEnemySeePlayer)
    (if (and (Variables|Default|GetCanAttack?) (not (Variables|Default|GetPlayingAnimation)))
      (AI|AIMoveTo self "0, 0, 0" (Game|GetPlayerCharacter 0) 5.0 false))))

(event EventBeginPlay
  ;[1 1 1] Events
  (Utilities|FlowControl|Sequence
    (:then_0
      (CallFunction|UpdateHealth))
    (:then_1
      (CallFunction|AddWeapon))))

(event EventTick
  (params (DeltaSeconds :type Float%20%28single-precision%29))
  (bind _returnvalue (Transformation|GetActorLocation))
  ;[1 1 1] Events
  (Utilities|FlowControl|Sequence
    (:then_0
      (CallFunction|MovetoPlayer))
    (:then_1
      ;[1 1 1] enemy attacks If player in trace
      (bind (_outhit _returnvalue_2) (Collision|LineTraceForObjects _returnvalue (+ _returnvalue (* (Transformation|GetActorForwardVector) 125.0)) (Utilities|Array|MakeArray "ObjectTypeQuery3") false 0 "None"))
      (if _returnvalue_2
        (Utilities|Casting|CastToPlayerCharacter1 (.HitActor (Collision|BreakHitResult _outhit)))
        (CallFunction|Attack)))))

(event EventDealingDamage
  (params (Damage :type Float%20%28single-precision%29) (Sneder :type Actor%20Object%20Reference))
  ;[1 1 1] Health and Damage
  (Variables|Default|SetCurrentHealth (- (Variables|Default|GetCurrentHealth) Damage))
  (CallFunction|UpdateHealth)
  (Utilities|FlowControl|Sequence
    (:then_0
      (Variables|Default|SetPlayingAnimation true)
      (Utilities|FlowControl|Delay 0.2)
      (Variables|Default|SetPlayingAnimation false))
    (:then_1
      (Audio|PlaySoundatLocation "/Game/Assets/Audio/Attack.Attack" (Transformation|GetActorLocation) "0, 0, 0" 1.0 1.0 0.0 0 0 0))))

(fn ConstructionScript)

(fn UpdateHealth
  (bind _asenemy_health (Utilities|Casting|CastToEnemy_Health (UserInterface|GetUserWidgetObject (Variables|Default|GetEnemyHealth))))
  (Progress|SetPercent (Variables|/Game/Blueprints/Enemys/Enemy_Health.Enemy_Health_C|GetHealth _asenemy_health) (/ (Variables|Default|GetCurrentHealth) (Variables|Default|GetMaxHealth)))
  (if (<= (Variables|Default|GetCurrentHealth) 0.0)
    (CallFunction|Death))
  (return))

(fn Death
  (if (<= (Variables|Default|GetCurrentHealth) 0.0)
    (Physics|SetSimulatePhysics (Variables|Character|GetMesh) true)
    (Rendering|SetVisibility (Variables|Default|GetEnemyHealth) false false)
    (Collision|SetCollisionEnabled (Variables|Collision|GetCapsuleComponent) "NoCollision")
    (Variables|Default|SetEnemyDeath true)
    (Class|KismetSystemLibrary|PauseTimer (Variables|Default|GetEnemySwordRef) "AttackTrace")
    (return)))